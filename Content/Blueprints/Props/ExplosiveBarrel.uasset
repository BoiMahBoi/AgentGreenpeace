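; Explosive barrel prop that loses health when damaged and explodes once it reaches zero.
; The explosion fires only once, deactivating the mesh component, spiking the point light and activating a Niagara effect.
; A sphere overlap around the barrel finds pawns and damages those derived from BP_Creature, then the actor destroys itself after a short delay.
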(event `self.Take Damage`
  (params (Damage :type Integer))
  (bind _output_get (set `self.Health` (- (`self.Health`) Damage)))
  (if (<= _output_get 0)
    (`self.Explode`)))

(event `Explode`
  (if (not (`self.hasExploded`))
    (`ActorComponent.SetActive` (`self.StaticMesh`) false false)
    (set `self.hasExploded` true)
    (`LightComponent.SetIntensity` (`self.PointLight`) 10000.0)
    (`ActorComponent.Activate` (`self.Niagara`) false)
    (bind _outactors (`KismetSystemLibrary.SphereOverlapActors` (`self.K2_GetActorLocation`) 300.0 (`|MakeArray` "ObjectTypeQuery3" :!type "EObjectTypeQuery Enum")))
    (for _array_element _outactors
      (if (`KismetMathLibrary.ClassIsChildOf` (`GameplayStatics.GetObjectClass` _array_element) "/Game/Blueprints/Enemies/BP_Creature.BP_Creature_C")
        (bind _asbp_creature (cast `/Game/Blueprints/Enemies/BP_Creature` _array_element))
        (`self.Take Damage` _asbp_creature 30)))
    (`KismetSystemLibrary.Delay` 0.5)
    (`self.K2_DestroyActor`)))

(fn `UserConstructionScript`)