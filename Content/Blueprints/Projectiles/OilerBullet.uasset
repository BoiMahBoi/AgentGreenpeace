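; OilerBullet is a projectile Blueprint that damages the player on contact.
; Its construction script calls the parent's, then sets the projectile damage.
; When its box collision overlaps player character 0, it casts that character to BP_Creature, calls TakeDamage with that damage and prints a debug message.
; A DestroyActor node is left unconnected, so this graph does not destroy the bullet on hit.
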(event `self.BoxCollision.OnComponentBeginOverlap`
  (params (OverlappedComponent :type "PrimitiveComponent Object Reference") (OtherActor :type "Actor Object Reference") (OtherComp :type "PrimitiveComponent Object Reference") (OtherBodyIndex :type Integer) (bFromSweep :type Boolean) (SweepResult :type "HitResult Structure (by ref)"))
  (bind _returnvalue (`GameplayStatics.GetPlayerCharacter` 0))
  (`|ExecutionSequence`
    (:`then_0`
      (if (== OtherActor _returnvalue)
        (bind _asbp_creature (cast `/Game/Blueprints/Enemies/BP_Creature` _returnvalue))
        (`/Game/Blueprints/Enemies/BP_Creature.Take Damage` _asbp_creature (`self.ProjectileDamage`))
        (`KismetSystemLibrary.PrintString` "Take Damage!")))))

(fn `UserConstructionScript`
  (`parent.UserConstructionScript`)
  (set `self.ProjectileDamage` 10))