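; BP_Raygun is a hitscan gun for the first-person player, with a cooldown between shots.
; Shoot plays a pitch-randomized sound, muzzle flash, screen-flash widget and pitch kick, then line traces from the camera with debug drawing.
; A Sequence casts the hit actor to BP_Oiler and BP_Gasser to apply slightly randomized damage, then re-enables firing after a Delay.
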(event `self.ReceiveBeginPlay`
  (bind _asbp_first_person_character (cast `/Game/Blueprints/PlayerController/BP_FirstPersonCharacter` (`GameplayStatics.GetPlayerCharacter` 0))))

(event `Shoot`
  (bind _damage (`self.Damage`))
  (bind _returnvalue (`KismetMathLibrary.RandomIntegerInRange` (- _damage 5) (+ _damage 5)))
  (if (`self.CanShoot`)
    (set `self.CanShoot` false)
    (`GameplayStatics.PlaySound2D` "/Game/Audio/Pistol_Sound.Pistol_Sound" 1.0 (`KismetMathLibrary.RandomFloatInRange` 0.9 1.1) 0.0 null null)
    (`GameplayStatics.SpawnEmitterAtLocation` "/Game/Particles/MuzzleFlash.MuzzleFlash" (`SceneComponent.K2_GetComponentLocation` (`self.Arrow`)) (`self.K2_GetActorRotation`))
    (`self.FlashGun`)
    (`self.KickGun` (stale `self.ReceiveBeginPlay` _asbp_first_person_character))
    (bind _firstpersoncamera (`/Game/Blueprints/PlayerController/BP_FirstPersonCharacter.FirstPersonCamera` (stale `self.ReceiveBeginPlay` _asbp_first_person_character)))
    (bind _returnvalue_2 (`SceneComponent.K2_GetComponentLocation` _firstpersoncamera))
    (bind _outhit (`KismetSystemLibrary.LineTraceSingle` :`Start` _returnvalue_2 :`End` (+ _returnvalue_2 (* (`KismetMathLibrary.GetForwardVector` (`SceneComponent.K2_GetComponentRotation` _firstpersoncamera)) (`self.Range`))) :`TraceChannel` "TraceTypeQuery1" :`DrawDebugType` "ForDuration" :`DrawTime` 1.0))
    (`|ExecutionSequence`
      (:`then_0`
        (bind (_bblockinghit _binitialoverlap _time _distance _location _impactpoint _normal _impactnormal _physmat _hitactor) (`GameplayStatics.BreakHitResult` _outhit))
        (bind _asbp_oiler (cast `/Game/Blueprints/Enemies/Oiler/BP_Oiler` _hitactor))
        (`/Game/Blueprints/Enemies/Oiler/BP_Oiler.Take Damage` _asbp_oiler _returnvalue))
      (:`then_1`
        (bind _asbp_gasser (cast `/Game/Blueprints/Enemies/Gasser/BP_Gasser` _hitactor))
        (`/Game/Blueprints/Enemies/Gasser/BP_Gasser.Take Damage` _asbp_gasser _returnvalue))
      (:`then_2`
        (`KismetSystemLibrary.Delay` (`self.Cooldown`))
        (set `self.CanShoot` true)))
    (else
      (`KismetSystemLibrary.PrintString` "Can't shoot!"))))

(fn `FlashGun`
  (bind _returnvalue (`|CreateWidget` "/Game/Blueprints/UI/ShootFlash.ShootFlash_C"))
  (`UserWidget.AddToViewport` _returnvalue 0))

(fn `KickGun`
  (params (`Character Ref` :type "Actor Object Reference"))
  (`Pawn.AddControllerPitchInput` (`Actor.Instigator` `Character Ref`) (`self.Kick`)))

(fn `UserConstructionScript`)