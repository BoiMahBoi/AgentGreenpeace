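; BP_Strawgun is a hitscan gun fired from the first-person player's camera, damaging any BP_Creature it hits.
; Shoot is gated by ammo and a cooldown flag, then plays pitch-varied sound, muzzle flash, a screen flash widget and pitch recoil.
; A visibility line trace places a short-lived bullet decal and applies slightly randomized damage.
; The construction script fills ammo to maximum; debug trace drawing and an ammo print remain active.
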(event `self.ReceiveBeginPlay`
  (bind _asbp_first_person_character (cast `/Game/Blueprints/PlayerController/BP_FirstPersonCharacter` (`GameplayStatics.GetPlayerCharacter` 0))))

(event `Shoot`
  (bind _damage (`self.Damage`))
  (if (`self.CanShoot`)
    (if (> (`self.CurrentAmmo`) 0)
      (`self.LoseAmmo` 1)
      (`KismetSystemLibrary.PrintString` (`KismetStringLibrary.Conv_IntToString` (`self.CurrentAmmo`)))
      (set `self.CanShoot` false)
      (`GameplayStatics.PlaySound2D` "/Game/Audio/Pistol_Sound.Pistol_Sound" 1.0 (`KismetMathLibrary.RandomFloatInRange` 0.9 1.1) 0.0 null null)
      (`GameplayStatics.SpawnEmitterAtLocation` "/Game/Particles/MuzzleFlash.MuzzleFlash" (`SceneComponent.K2_GetComponentLocation` (`self.Arrow`)) (`self.K2_GetActorRotation`))
      (`self.FlashGun`)
      (`self.KickGun` (stale `self.ReceiveBeginPlay` _asbp_first_person_character))
      (bind _firstpersoncamera (`/Game/Blueprints/PlayerController/BP_FirstPersonCharacter.FirstPersonCamera` (stale `self.ReceiveBeginPlay` _asbp_first_person_character)))
      (bind _returnvalue (`SceneComponent.K2_GetComponentLocation` _firstpersoncamera))
      (bind _outhit (`KismetSystemLibrary.LineTraceSingle` :`Start` _returnvalue :`End` (+ _returnvalue (* (`KismetMathLibrary.GetForwardVector` (`SceneComponent.K2_GetComponentRotation` _firstpersoncamera)) (`self.Range`))) :`TraceChannel` "TraceTypeQuery1" :`DrawDebugType` "ForDuration" :`DrawTime` 1.0))
      (`|ExecutionSequence`
        (:`then_0`
          (bind (_bblockinghit _binitialoverlap _time _distance _location _impactpoint _normal _impactnormal _physmat _hitactor) (`GameplayStatics.BreakHitResult` _outhit))
          (`GameplayStatics.SpawnDecalAtLocation` "/Game/Materials/BulletDecalMat.BulletDecalMat" (20.0 20.0 20.0) _location (`KismetMathLibrary.Conv_VectorToRotator` _impactnormal) 5.0)
          (bind _asbp_creature (cast `/Game/Blueprints/Enemies/BP_Creature` _hitactor))
          (`/Game/Blueprints/Enemies/Oiler/BP_Oiler.Take Damage` _asbp_creature (`KismetMathLibrary.RandomIntegerInRange` (- _damage 5) (+ _damage 5))))
        (:`then_1`
          (`KismetSystemLibrary.Delay` (`self.Cooldown`))
          (set `self.CanShoot` true))))))

(fn `FlashGun`
  (bind _returnvalue (`|CreateWidget` "/Game/Blueprints/UI/ShootFlash.ShootFlash_C"))
  (`UserWidget.AddToViewport` _returnvalue 0))

(fn `KickGun`
  (params (`Player Character Ref` :type "Actor Object Reference"))
  (`Pawn.AddControllerPitchInput` (`Actor.Instigator` `Player Character Ref`) (`self.Kick`)))

(fn `UserConstructionScript`
  (bind _output_get (set `self.MaxAmmo` 200))
  (set `self.CurrentAmmo` _output_get))