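; BP_Weapon is a weapon Blueprint that tracks an ammo count.
; The PickupAmmo event adds ammo, caps it at MaxAmmo and prints the resulting count.
; The LoseAmmo function subtracts a given amount and floors the count at zero.
; It contains no firing logic, and nothing in its graphs calls LoseAmmo.
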(event `PickupAmmo`
  (params (Ammo :type Integer))
  (bind _maxammo (`self.MaxAmmo`))
  (bind _output_get (set `self.CurrentAmmo` (+ (`self.CurrentAmmo`) Ammo)))
  (if (> _output_get _maxammo)
    (bind _output_get_2 (set `self.CurrentAmmo` _maxammo))
    (`KismetSystemLibrary.PrintString` (`KismetStringLibrary.Conv_IntToString` _output_get_2))
    (else
      (`KismetSystemLibrary.PrintString` (`KismetStringLibrary.Conv_IntToString` _output_get)))))

(fn `LoseAmmo`
  (params (AmmoAmount :type Integer))
  (bind _output_get (set `self.CurrentAmmo` (- (`self.CurrentAmmo`) AmmoAmount)))
  (if (< _output_get 0)
    (set `self.CurrentAmmo` 0)))

(fn `UserConstructionScript`)