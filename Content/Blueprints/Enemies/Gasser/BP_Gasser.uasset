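; BP_Gasser is an exploding enemy that spawns a GasserExplosion at its location and destroys itself.
; It detonates when the first-person character enters its RangeCollider or when damage drains its health, which is initialized in the construction script.
; PawnSensing sets the IsPlayerSeen blackboard key on its AI controller when it sees the player.
; Debug prints remain on the hit and overlap events.
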(event `Take Damage`
  (params (Damage :type Integer))
  (`KismetSystemLibrary.PrintString` "Hit!")
  (bind _output_get (set `self.CurrentHealth` (- (`self.CurrentHealth`) Damage)))
  (if (<= _output_get 0)
    (`|SpawnActorFromClass` "/Game/Blueprints/Enemies/Gasser/GasserExplosion.GasserExplosion_C" (`self.GetTransform`) "Undefined" "MultiplyWithRoot" null null)
    (`self.K2_DestroyActor`)))

(event `self.PawnSensing.OnSeePawn`
  (params (Pawn :type "Pawn Object Reference"))
  (if (== Pawn (`GameplayStatics.GetPlayerPawn` 0))
    (`BlackboardComponent.SetValueAsBool` (`AIBlueprintHelperLibrary.GetBlackboard` (`AIBlueprintHelperLibrary.GetAIController` self)) "IsPlayerSeen" true)))

(event `self.RangeCollider.OnComponentBeginOverlap`
  (params (OverlappedComponent :type "PrimitiveComponent Object Reference") (OtherActor :type "Actor Object Reference") (OtherComp :type "PrimitiveComponent Object Reference") (OtherBodyIndex :type Integer) (bFromSweep :type Boolean) (SweepResult :type "HitResult Structure (by ref)"))
  (cast `/Game/Blueprints/PlayerController/BP_FirstPersonCharacter` OtherActor)
  (`|SpawnActorFromClass` "/Game/Blueprints/Enemies/Gasser/GasserExplosion.GasserExplosion_C" (`self.GetTransform`) "AlwaysSpawn" "MultiplyWithRoot" null null)
  (`KismetSystemLibrary.PrintString` "Hello")
  (`self.K2_DestroyActor`))

(fn `UserConstructionScript`
  (set `self.CurrentHealth` 30))