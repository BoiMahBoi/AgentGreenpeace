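; BP_Oiler is an enemy Blueprint with basic health and player detection for an AI controller.
; Health starts at its maximum, drops with incoming damage and destroys the actor at zero or below.
; PawnSensing checks whether a seen pawn is the first player and, if so, sets the IsPlayerSeen blackboard flag, which this file never clears.
; Both hits and sightings print debug strings.
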(event `self.ReceiveBeginPlay`
  (set `self.CurrentHealth` (`self.MaxHealth`)))

(event `Take Damage`
  (params (Damage :type Integer))
  (bind _currenthealth (`self.CurrentHealth`))
  (`KismetSystemLibrary.PrintString` "Hit!")
  (set `self.CurrentHealth` (- _currenthealth Damage))
  (if (<= _currenthealth 0)
    (`self.K2_DestroyActor`)))

(event `self.PawnSensing.OnSeePawn`
  (params (Pawn :type "Pawn Object Reference"))
  (if (== Pawn (`GameplayStatics.GetPlayerPawn` 0))
    (`KismetSystemLibrary.PrintString` "Player seen")
    (`BlackboardComponent.SetValueAsBool` (`AIBlueprintHelperLibrary.GetBlackboard` (`AIBlueprintHelperLibrary.GetAIController` self)) "IsPlayerSeen" true)))

(fn `UserConstructionScript`)