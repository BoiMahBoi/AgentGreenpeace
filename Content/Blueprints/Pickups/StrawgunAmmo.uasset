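; Strawgun ammo pickup that tops up the Strawgun when the player walks into it.
; It spins slowly in yaw on Tick by a fixed per-frame step, not scaled by delta time.
; On overlap with the first-person player character, it calls PickupAmmo with a fixed amount on the BP_Strawgun found by GetActorOfClass, then destroys itself.
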(event `self.ReceiveTick`
  (params (DeltaSeconds :type "Float (single-precision)"))
  (`self.K2_AddActorWorldRotation` (`KismetMathLibrary.MakeRotator` 0.0 0.0 0.25)))

(event `self.ReceiveActorBeginOverlap`
  (params (OtherActor :type "Actor Object Reference"))
  (if (== OtherActor (`GameplayStatics.GetPlayerPawn` 0))
    (cast `/Game/Blueprints/PlayerController/BP_FirstPersonCharacter` (`GameplayStatics.GetPlayerCharacter` 0))
    (bind _returnvalue (`GameplayStatics.GetActorOfClass` "/Game/Blueprints/Weapons/BP_Strawgun.BP_Strawgun_C"))
    (`/Game/Blueprints/Weapons/BP_Weapon.PickupAmmo` _returnvalue 5)
    (`self.K2_DestroyActor`)))

(fn `UserConstructionScript`)